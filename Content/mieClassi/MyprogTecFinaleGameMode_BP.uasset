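; Game mode Blueprint that respawns the player's third-person character after it is destroyed.
; On BeginPlay it binds a handler to the character's OnDestroyed event.
; When that fires, it waits briefly, spawns a new character at the stored SpawnLocation and has the first player controller possess it.
; It then calls Respawn to bind the handler to the new character, so the cycle repeats.
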(event `Respawn`
  (bind _asthird_person_character (cast `/Game/ThirdPersonCPP/Blueprints/ThirdPersonCharacter` (`GameplayStatics.GetPlayerCharacter` 0) :!label _label))
  (add `Actor.OnDestroyed` _asthird_person_character (delegate `CustomEvent`)))

(event `self.ReceiveBeginPlay`
  (goto _label))

(event `CustomEvent`
  (params (DestroyedActor :type "Actor Object Reference"))
  (`KismetSystemLibrary.Delay` 2.0)
  (bind _returnvalue (`|SpawnActorFromClass` "/Game/ThirdPersonCPP/Blueprints/ThirdPersonCharacter.ThirdPersonCharacter_C" (`self.Spawn Location`) "AdjustIfPossibleButAlwaysSpawn" "OverrideRootScale" null null))
  (`Controller.Possess` (`GameplayStatics.GetPlayerController` 0) _returnvalue)
  (`self.Respawn`))

(fn `UserConstructionScript`)